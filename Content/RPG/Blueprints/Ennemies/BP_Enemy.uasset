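; BP_Enemy is an RPG enemy with a life pool that drains when it takes damage.
; On spawn it fills its life and caches the player as BP_Player.
; At zero life it notifies the player's QuestsManager to check kill objectives, then destroys itself after a short delay.
; U key bindings, one of them a debug key, trigger the same death path directly.
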(event EventBeginPlay
  (Variables|Default|SetCurrentLife (Variables|Default|GetMaxLife))
  (bind _asbp_player (Utilities|Casting|CastToBP_Player (Game|GetPlayerCharacter 0)))
  (Variables|Default|SetBP%20Player _asbp_player))

(event Game|Damage|EventAnyDamage
  (params (Damage :type Float%20%28single-precision%29) (DamageType :type Damage%20Type%20Object%20Reference) (InstigatedBy :type Controller%20Object%20Reference) (DamageCauser :type Actor%20Object%20Reference))
  (bind _output_get (Variables|Default|SetCurrentLife (- (Variables|Default|GetCurrentLife) Damage)))
  (if (<= _output_get 0.0)
    (Default|CheckKillObjectives (Variables|/Game/RPG/Player/BP_Player.BP_Player_C|GetQuestsManager (Variables|Default|GetBP%20Player)) self)
    (Utilities|FlowControl|Delay 0.1)
    (Actor|DestroyActor)))

(event Input|KeyboardEvents|DebugKeyU
  (params (Key :type Key%20Structure) (ActionValue :type Input%20Action%20Value%20Structure))
  (:Pressed
    (Default|CheckKillObjectives (Variables|/Game/RPG/Player/BP_Player.BP_Player_C|GetQuestsManager (Variables|Default|GetBP%20Player)) self)
    (Utilities|FlowControl|Delay 0.1)
    (Actor|DestroyActor)))

(event Input|KeyboardEvents|U
  (params (Key :type Key%20Structure))
  (:Pressed
    (Default|CheckKillObjectives (Variables|/Game/RPG/Player/BP_Player.BP_Player_C|GetQuestsManager (Variables|Default|GetBP%20Player)) self)
    (Utilities|FlowControl|Delay 0.1)
    (Actor|DestroyActor)))

(fn ConstructionScript)