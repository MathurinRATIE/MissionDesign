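; BP_Item is a world pickup that shows its item data's mesh and can optionally self-destruct on a timer.
; When the player overlaps it, it adds its amount to their inventory, destroying itself on success or keeping what was not added.
; A looping timer polls physics velocity until nearly zero, then disables simulation and starts timeline-driven spin and vertical bobbing.
; A leftover "Vif d'Or Glitch" section holds world-space variants of that animation.
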(event `self.ReceiveBeginPlay`
  (`StaticMeshComponent.SetStaticMesh` (`self.StaticMesh`) (`/Game/RPG/Blueprints/Item/ItemsDatas/PDA_ItemDatas.Mesh` (`self.ItemDatas`)))
  (`self.CheckFloatingActivation`)
  (if (`self.ShouldSelfDestruct`)
    (`self.SelfDestruct`)))

(event `self.PickupCollision.OnComponentBeginOverlap`
  (params (OverlappedComponent :type "PrimitiveComponent Object Reference") (OtherActor :type "Actor Object Reference") (OtherComp :type "PrimitiveComponent Object Reference") (OtherBodyIndex :type Integer) (bFromSweep :type Boolean) (SweepResult :type "HitResult Structure (by ref)"))
  (if (`self.ActorHasTag` OtherActor "Player")
    (bind _asbp_player (cast `/Game/RPG/Player/BP_Player` OtherActor))
    (bind (_bool _amountnotadded) (`/Game/RPG/Player/Components/BPC_Inventory.AddItem` (`/Game/RPG/Player/BP_Player.PBC_Inventory` _asbp_player) (`self.ItemDatas`) (`self.Amount`)))
    (if _bool
      (`self.K2_DestroyActor`)
      (else
        (set `self.Amount` _amountnotadded)))))

(event `SelfDestruct`
  (`KismetSystemLibrary.K2_SetTimerDelegate` (delegate `Destroy`) 300.0))

(event `Destroy`
  (`self.K2_DestroyActor`))

(event `CheckFloatingActivation`
  ;[0.05098 0.05098 0.05098] Flotting items
  (bind _returnvalue (`KismetSystemLibrary.K2_SetTimerDelegate` (delegate `Check Grounded`) 0.01 true))
  (set `self.FallingStopLoop` _returnvalue))

(event `Check Grounded`
  ;[0.05098 0.05098 0.05098] Flotting items
  (if (`KismetMathLibrary.Vector_IsNearlyZero` (`SceneComponent.GetComponentVelocity` (`self.PhysicCollision`)) 1.0)
    (`PrimitiveComponent.SetSimulatePhysics` (`self.PhysicCollision`) false)
    (`self.Rotate`)
    (`self.MoveUpDown`)
    (`KismetSystemLibrary.K2_ClearAndInvalidateTimerHandle` (`self.FallingStopLoop`))))

(event `MoveUpDown`
  (bind _staticmesh (`self.StaticMesh`))
  (bind (_relativelocation_x _relativelocation_y) (`KismetMathLibrary.BreakVector` (`SceneComponent.RelativeLocation` _staticmesh)))
  ;[0.05098 0.05098 0.05098] Flotting items
  (bind (_direction _time) (`Timeline|UpDownTimeline` :!label _label)
    (:`Update`
      (`SceneComponent.K2_SetRelativeLocation` _staticmesh (`KismetMathLibrary.MakeVector` _relativelocation_x _relativelocation_y (* _time 50.0)) false false))
    (:`Finished`
      (if (< _time 0.5)
        (goto _label :!via `PlayFromStart`)
        (else
          (goto _label :!via `ReverseFromEnd`))))))

(event `Rotate`
  (bind _staticmesh (`self.StaticMesh`))
  (bind (_relativerotation_roll _relativerotation_pitch) (`KismetMathLibrary.BreakRotator` (`SceneComponent.RelativeRotation` _staticmesh)))
  ;[0.05098 0.05098 0.05098] Flotting items
  (bind (_direction _time) (`Timeline|RotateTimeline` :!label _label_2)
    (:`Update`
      (`SceneComponent.K2_SetRelativeRotation` _staticmesh (`KismetMathLibrary.MakeRotator` _relativerotation_roll _relativerotation_pitch (* _time 360.0)) false false))
    (:`Finished`
      (`self.ContinueRotrate`))))

(event `ContinueRotrate`
  ;[0.05098 0.05098 0.05098] Flotting items
  (goto _label_2 :!via `PlayFromStart`))

(event `CustomEvent_2`
  (bind _staticmesh (`self.StaticMesh`))
  (bind (_returnvalue_roll _returnvalue_pitch) (`KismetMathLibrary.BreakRotator` (`SceneComponent.K2_GetComponentRotation` _staticmesh)))
  ;[0.05098 0.05098 0.05098] Vif d'Or Glitch
  (bind (_direction _time) (`Timeline|Timeline_0` :!via `PlayFromStart`)
    (:`Update`
      (`SceneComponent.K2_SetWorldRotation` _staticmesh (`KismetMathLibrary.MakeRotator` _returnvalue_roll _returnvalue_pitch (+ (* _time 360.0) 0.0)) false false))
    (:`Finished`
      (`self.ContinueRotrate`))))

(fn `UserConstructionScript`)