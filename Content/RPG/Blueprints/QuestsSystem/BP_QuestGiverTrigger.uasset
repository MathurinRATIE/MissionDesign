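; Quest giver trigger volume that plays a sequence of dialogue lines when the player enters it, then grants a quest.
; Overlap hides the in-game HUD, shows the dialogue widget with cursor and UI-only input, and hands it a reference to this trigger.
; NextDialogue steps through the Dialogues array.
; After the last line it restores HUD and game input, claims the quest through the player's QuestsManager and destroys itself.
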(event `self.ReceiveBeginPlay`
  (bind _aspc_player (cast `/Game/RPG/_Common/PC_Player` (`GameplayStatics.GetPlayerController` 0)))
  (set `self.PC Player` _aspc_player))

(event `self.QuestGiverBox.OnComponentBeginOverlap`
  (params (OverlappedComponent :type "PrimitiveComponent Object Reference") (OtherActor :type "Actor Object Reference") (OtherComp :type "PrimitiveComponent Object Reference") (OtherBodyIndex :type Integer) (bFromSweep :type Boolean) (SweepResult :type "HitResult Structure (by ref)"))
  (if (and (`self.ActorHasTag` OtherActor "Player") (not (`self.QuestGiven`)))
    (`self.StartDialogue`)))

(fn `DisplayDialogue`
  (set `TextBlock.Text` (`|GetArrayItem` (`self.Dialogues`) (`self.CurrentDialogue`)) (`/Game/RPG/UI/Dialogue/WBP_InfoDialogue.Dialogue` (`/Game/RPG/_Common/PC_Player.WBP_InfoDialogue` (`self.PC Player`)))))

(fn `EndDialogue`
  (`Widget.SetVisibility` (`/Game/RPG/_Common/PC_Player.WBP_InGame` (`self.PC Player`)) "Visible")
  (`Widget.SetVisibility` (`/Game/RPG/_Common/PC_Player.WBP_InfoDialogue` (`self.PC Player`)) "Hidden")
  (`/Game/RPG/Blueprints/QuestsSystem/BP_QuestsManager.ClaimQuest` (`/Game/RPG/Player/BP_Player.QuestsManager` (`/Game/RPG/_Common/PC_Player.BP Player` (`self.PC Player`))) (`self.QuestDatas`))
  (set `PlayerController.bShowMouseCursor` false (`self.PC Player`))
  (`WidgetBlueprintLibrary.SetInputMode_GameOnly` (`self.PC Player`))
  (`self.K2_DestroyActor`))

(fn `NextDialogue`
  (bind _result (`/Engine/EditorBlueprintResources/StandardMacros.IncrementInt` (`self.CurrentDialogue`))
    (:`  `
      (if (< _result (`KismetArrayLibrary.Array_Length` (`self.Dialogues`)))
        (`self.DisplayDialogue`)
        (else
          (`self.EndDialogue`))))))

(fn `StartDialogue`
  (bind (_returnvalue_x _returnvalue_y) (`KismetMathLibrary.BreakVector2D` (`WidgetLayoutLibrary.GetViewportSize`)))
  (`Widget.SetVisibility` (`/Game/RPG/_Common/PC_Player.WBP_InGame` (`self.PC Player`)) "Hidden")
  (`Widget.SetVisibility` (`/Game/RPG/_Common/PC_Player.WBP_InfoDialogue` (`self.PC Player`)) "Visible")
  (`self.DisplayDialogue`)
  (`PlayerController.SetMouseLocation` (`self.PC Player`) (`KismetMathLibrary.FTrunc` (* _returnvalue_x 0.5)) (`KismetMathLibrary.FTrunc` (- _returnvalue_y 450.0)))
  (set `PlayerController.bShowMouseCursor` true (`self.PC Player`))
  (`WidgetBlueprintLibrary.SetFocusToGameViewport`)
  (`WidgetBlueprintLibrary.SetInputMode_UIOnlyEx` (`self.PC Player`) (`/Game/RPG/_Common/PC_Player.WBP_InfoDialogue` (`self.PC Player`)))
  (set `/Game/RPG/UI/Dialogue/WBP_InfoDialogue.QuestTrigger` self (`/Game/RPG/_Common/PC_Player.WBP_InfoDialogue` (`self.PC Player`))))

(fn `UserConstructionScript`)