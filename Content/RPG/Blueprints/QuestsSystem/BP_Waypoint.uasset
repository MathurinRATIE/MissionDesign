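; Quest waypoint actor that marks a location objective and reports to the player's QuestsManager when reached.
; QuestsManager events activate or deactivate it by ID, toggling a widget marker whose distance to the player updates on Tick.
; Approximate objectives show a zone decal sized with the trigger box and can require staying inside for a Tick-driven countdown, shown on screen.
; Leaving before the countdown ends resets it and restores the marker.
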(event `self.ReceiveTick`
  (params (DeltaSeconds :type "Float (single-precision)"))
  (bind (_returnvalue_x _returnvalue_y) (`KismetMathLibrary.BreakVector` (`self.K2_GetActorLocation`)))
  (bind _as_wbp_waypoint (`self.As WBP Waypoint`))
  (bind (_returnvalue_x_2 _returnvalue_y_2) (`KismetMathLibrary.BreakVector` (`self.K2_GetActorLocation` (`self.BP Player`))))
  (bind _returnvalue (- (`KismetMathLibrary.Round` (/ (`KismetMathLibrary.Distance2D` (`KismetMathLibrary.MakeVector2D` _returnvalue_x _returnvalue_y) (`KismetMathLibrary.MakeVector2D` _returnvalue_x_2 _returnvalue_y_2)) 100.0)) 1))
  ;[1 1 1] Tick
  ;;[1 0.6649 0.2546] Set waypoint Distance
  (`/Engine/EditorBlueprintResources/StandardMacros.IsValid` (`self.As WBP Waypoint`)
    (:`Is Valid`
      (if (< _returnvalue 0)
        (set `/Game/RPG/UI/InGame/WBP_Waypoint.DistanceToTarget` 0.0 _as_wbp_waypoint)
        (else
          (set `/Game/RPG/UI/InGame/WBP_Waypoint.DistanceToTarget` (`KismetMathLibrary.Conv_IntToDouble` _returnvalue) _as_wbp_waypoint)))
      (if (`self.ExecuteTimer`)
        (`self.Countdown`)))))

(event `self.ReceiveBeginPlay`
  ;[1 1 1] Begin Play
  (bind _asbp_player (cast `/Game/RPG/Player/BP_Player` (`GameplayStatics.GetPlayerCharacter` 0)))
  (bind _output_get (set `self.BP Player` _asbp_player))
  (`KismetSystemLibrary.DelayUntilNextTick`)
  (add `/Game/RPG/Blueprints/QuestsSystem/BP_QuestsManager.ActivateWaypointOfID` (`/Game/RPG/Player/BP_Player.QuestsManager` _output_get) (delegate `waypoint_Event`))
  (set `self.Timer` (`self.maxTime`))
  (add `/Game/RPG/Blueprints/QuestsSystem/BP_QuestsManager.DeactivateWaypointOfID` (`/Game/RPG/Player/BP_Player.QuestsManager` (`self.BP Player`)) (delegate `DeactivateWaypoint`)))

(event `DeactivateWaypoint`
  (params (Id :type Integer))
  ;[1 1 1] Begin Play
  (if (== Id (`self.ID`))
    (set `self.Active` false)
    (`SceneComponent.SetVisibility` (`self.Decal`) false false)
    (`WidgetComponent.SetWidget` (`self.Widget`) null)))

(event `waypoint_Event`
  (params (id :type Integer))
  ;[1 1 1] Begin Play
  (if (== id (`self.ID`))
    (set `self.Active` true)
    (bind _returnvalue (`|CreateWidget` "/Game/RPG/UI/InGame/WBP_Waypoint.WBP_Waypoint_C"))
    (`WidgetComponent.SetWidget` (`self.Widget`) _returnvalue)
    (bind _aswbp_waypoint (cast `/Game/RPG/UI/InGame/WBP_Waypoint` (`WidgetComponent.GetWidget` (`self.Widget`))))
    (set `self.As WBP Waypoint` _aswbp_waypoint)
    (if (`self.ApproximateObjective`)
      (`SceneComponent.SetVisibility` (`self.Decal`) true false)
      (else
        (`SceneComponent.SetVisibility` (`self.Decal`) false false)))))

(event `self.WaypointDetection.OnComponentBeginOverlap`
  (params (OverlappedComponent :type "PrimitiveComponent Object Reference") (OtherActor :type "Actor Object Reference") (OtherComp :type "PrimitiveComponent Object Reference") (OtherBodyIndex :type Integer) (bFromSweep :type Boolean) (SweepResult :type "HitResult Structure (by ref)"))
  ;[1 1 1] On Overlap
  (if (`self.ActorHasTag` OtherActor "Player")
    (if (`self.Active`)
      (`/Engine/EditorBlueprintResources/StandardMacros.DoOnce` false :!label _label
        (:`Completed`
          (`DecalComponent.SetDecalMaterial` (`self.Decal`) "/Game/Materials/MI_ZoneInside.MI_ZoneInside")
          (`WidgetComponent.SetWidget` (`self.Widget`) null)
          (if (and (> (`self.Timer`) 0.0) (`self.ApproximateObjective`))
            (bind _returnvalue (`|CreateWidget` "/Game/RPG/UI/InGame/WBP_Timer.WBP_Timer_C" (`GameplayStatics.GetPlayerController` 0)))
            (bind _output_get (set `self.WBP Timer Widget` _returnvalue))
            (set `/Game/RPG/UI/InGame/WBP_Timer.Timer` (`KismetStringLibrary.TimeSecondsToString` (`self.Timer`)) _output_get)
            (`UserWidget.AddToViewport` _output_get 0)
            (`KismetSystemLibrary.Delay` 0.5)
            (set `self.ExecuteTimer` true)
            (else
              (`/Game/RPG/Blueprints/QuestsSystem/BP_QuestsManager.CheckLocationObjectives` (`/Game/RPG/Player/BP_Player.QuestsManager` (`self.BP Player`)) self)
              (`SceneComponent.SetVisibility` (`self.Decal`) false false)
              (set `self.QuestFinished` true))))))))

(event `ResetDoOnce`
  ;[1 1 1] On Overlap
  (goto _label :!via `Reset`))

(event `Countdown`
  ;[1 1 1] Zone Timer
  (bind _output_get (set `self.Timer` (`KismetMathLibrary.FClamp` (- (`self.Timer`) (`GameplayStatics.GetWorldDeltaSeconds`)) 0.0 (`self.Timer`))))
  (set `/Game/RPG/UI/InGame/WBP_Timer.Timer` (`KismetStringLibrary.TimeSecondsToString` _output_get) (`self.WBP Timer Widget`))
  (if (<= (`self.Timer`) 0.0)
    (set `self.ExecuteTimer` false)
    (`/Game/RPG/Blueprints/QuestsSystem/BP_QuestsManager.CheckLocationObjectives` (`/Game/RPG/Player/BP_Player.QuestsManager` (`self.BP Player`)) self)
    (`Widget.RemoveFromParent` (`self.WBP Timer Widget`))
    (`self.ResetDoOnce`)
    (`SceneComponent.SetVisibility` (`self.Decal`) false false)))

(event `self.WaypointDetection.OnComponentEndOverlap`
  (params (OverlappedComponent :type "PrimitiveComponent Object Reference") (OtherActor :type "Actor Object Reference") (OtherComp :type "PrimitiveComponent Object Reference") (OtherBodyIndex :type Integer))
  (bind _wbp_timer_widget (`self.WBP Timer Widget`))
  ;[1 1 1] When leaving trigger zone, check if there is a timer and reset it
  (if (`self.ActorHasTag` OtherActor "Player")
    (if (and (> (`self.Timer`) 0.0) (`self.Active`))
      (set `self.ExecuteTimer` false)
      (`self.ResetDoOnce`)
      (set `self.Timer` (`self.maxTime`))
      (set `self.Active` true)
      (`WidgetComponent.SetWidget` (`self.Widget`) (`self.As WBP Waypoint`))
      (`DecalComponent.SetDecalMaterial` (`self.Decal`) "/Game/Materials/MI_ZoneOutside.MI_ZoneOutside")
      (`/Engine/EditorBlueprintResources/StandardMacros.IsValid` _wbp_timer_widget
        (:`Is Valid`
          (`Widget.RemoveFromParent` _wbp_timer_widget))))))

(fn `UserConstructionScript`
  (bind (_collisionboxextent_x _collisionboxextent_y _collisionboxextent_z) (`KismetMathLibrary.BreakVector` (`self.CollisionBoxExtent`)))
  (`BoxComponent.SetBoxExtent` (`self.WaypointDetection`) (`self.CollisionBoxExtent`) true)
  (`SceneComponent.SetWorldScale3D` (`self.Decal`) (`KismetMathLibrary.MakeVector` _collisionboxextent_z _collisionboxextent_y _collisionboxextent_x)))