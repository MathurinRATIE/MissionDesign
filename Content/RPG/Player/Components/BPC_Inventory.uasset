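; Player inventory component that stores items as stacks in limited slots, with add, remove and capacity-check functions, the last simulating adds on a copy of the contents.
; Removal drains the newest slots first, and updates refresh the inventory widget and recheck collect quest objectives.
; Equip and UnEquip move items between inventory and equipment slots, adjusting armor points.
; Adding one special item ID raises Sympathy and animates its gauge with a looping timer.
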(event `self.ReceiveBeginPlay`
  (bind _foundwidgets (`WidgetBlueprintLibrary.GetAllWidgetsOfClass` "/Game/RPG/UI/Menu/Inventory/WBP_Inventory.WBP_Inventory_C" false))
  (set `self.WBP_Inventory` (`|GetArrayItem` _foundwidgets))
  (bind _asbp_player (cast `/Game/RPG/Player/BP_Player` (`self.GetOwner`)))
  (set `self.BP Player` _asbp_player))

(event `SympathyProgress`
  (params (PercentageToAdd :type "Float (double-precision)"))
  (bind _returnvalue (`KismetSystemLibrary.K2_SetTimerDelegate` (delegate `CustomTimeline`) 0.01 true))
  (set `self.Timer` _returnvalue))

(event `CustomTimeline`
  (bind _output_get (set `self.Time` (+ (`self.Time`) 0.01)))
  (`/Game/RPG/UI/WBP_SympathyJauge.PercentageIncrease` (`/Game/RPG/_Common/PC_Player.WBP_SympathyJauge` (`/Game/RPG/Player/BP_Player.PC Player` (`self.BP Player`))) (stale `SympathyProgress` PercentageToAdd) _output_get)
  (if (>= (`self.Time`) 1.0)
    (`KismetSystemLibrary.K2_ClearAndInvalidateTimerHandle` (`self.Timer`))))

(fn `AddItem`
  (params (Item :type "/Game/RPG/Blueprints/Item/ItemsDatas/PDA_ItemDatas Object Reference") (Count :type Integer))
  (returns (Bool :type "Object Object Reference") (AmountNotAdded :type Integer))
  (locals (AmountLeft :type Integer) (ItemToAdd :type "/Game/RPG/Blueprints/Item/ItemsDatas/PDA_ItemDatas Object Reference") (CurrentSlotID :type Integer) (CurrentSlotAmount :type Integer))
  (bind _itemtoadd (`local.ItemToAdd`))
  (bind _itemtoadd_2 (`local.ItemToAdd`))
  (bind (_output_item _output_amount) (break `/Game/RPG/Blueprints/Item/S_ItemSlot` (`|GetArrayItem` (`self.Content`) (`local.CurrentSlotID`))))
  (bind _stacksize (`/Game/RPG/Blueprints/Item/ItemsDatas/PDA_ItemDatas.StackSize` _itemtoadd))
  (bind _output_get (set `local.ItemToAdd` Item))
  (set `local.AmountLeft` Count)
  (if (not (not (== (`/Game/RPG/Blueprints/Item/ItemsDatas/PDA_ItemDatas.ID` _output_get) 123)))
    (bind _result (`/Engine/EditorBlueprintResources/StandardMacros.IncrementInt` (`self.Sympathy`))
      (:`  `
        (`self.SympathyProgress` (/ _result 10)))))
  (for _index (range (`KismetArrayLibrary.Array_Length` (`self.Content`)))
    (set `local.CurrentSlotID` _index)
    ;[0.05098 0.05098 0.05098] Add Item to Existing Slot
    (set `local.CurrentSlotAmount` _output_amount)
    (if (and (== _output_item _itemtoadd) (< (`local.CurrentSlotAmount`) _stacksize))
      (if (<= (+ (`local.CurrentSlotAmount`) (`local.AmountLeft`)) _stacksize)
        (`KismetArrayLibrary.Array_Set` (`self.Content`) (`local.CurrentSlotID`) (make `/Game/RPG/Blueprints/Item/S_ItemSlot` (`local.ItemToAdd`) (+ (`local.CurrentSlotAmount`) (`local.AmountLeft`))))
        (set `local.AmountLeft` 0)
        (break)
        (else
          (set `local.AmountLeft` (- (`local.AmountLeft`) (`/Game/RPG/Blueprints/Item/ItemsDatas/PDA_ItemDatas.StackSize` (`local.ItemToAdd`)) (`local.CurrentSlotAmount`)))
          (`KismetArrayLibrary.Array_Set` (`self.Content`) (`local.CurrentSlotID`) (make `/Game/RPG/Blueprints/Item/S_ItemSlot` (`local.ItemToAdd`) (`/Game/RPG/Blueprints/Item/ItemsDatas/PDA_ItemDatas.StackSize` (`local.ItemToAdd`))))))))
  ;[0.05098 0.05098 0.05098] Add Item to New Slot
  (if (== (`local.AmountLeft`) 0)
    (`self.UpdateWidget`)
    (return "true" 0)
    (else
      (if (< (`KismetArrayLibrary.Array_Length` (`self.Content`)) (`self.SlotsAmount`)) :!label _label
        (if (<= (`local.AmountLeft`) (`/Game/RPG/Blueprints/Item/ItemsDatas/PDA_ItemDatas.StackSize` (`local.ItemToAdd`)))
          (`KismetArrayLibrary.Array_Add` (`self.Content`) (make `/Game/RPG/Blueprints/Item/S_ItemSlot` (`local.ItemToAdd`) (`local.AmountLeft`)))
          (`self.UpdateWidget`)
          (return "true" 0)
          (else
            (`KismetArrayLibrary.Array_Add` (`self.Content`) (make `/Game/RPG/Blueprints/Item/S_ItemSlot` _itemtoadd_2 (`/Game/RPG/Blueprints/Item/ItemsDatas/PDA_ItemDatas.StackSize` _itemtoadd_2)))
            (set `local.AmountLeft` (- (`local.AmountLeft`) (`/Game/RPG/Blueprints/Item/ItemsDatas/PDA_ItemDatas.StackSize` (`local.ItemToAdd`))))
            (if (== (`local.AmountLeft`) 0)
              (`self.UpdateWidget`)
              (return "true" 0)
              (else
                (goto _label)))))
        (else
          (`self.UpdateWidget`)
          (return false (`local.AmountLeft`)))))))

(fn `AddItemToSpecificContent`
  (params (Item :type "/Game/RPG/Blueprints/Item/ItemsDatas/PDA_ItemDatas Object Reference") (Count :type Integer) (InputContent :type "Array of /Game/RPG/Blueprints/Item/S_ItemSlot Structure"))
  (returns (Bool :type "Object Object Reference") (OutputContent :type "Array of /Game/RPG/Blueprints/Item/S_ItemSlot Structure"))
  (locals (AmountLeft :type Integer) (ItemToAdd :type "/Game/RPG/Blueprints/Item/ItemsDatas/PDA_ItemDatas Object Reference") (CurrentSlotID :type Integer) (CurrentSlotAmount :type Integer) (LocalContent :type "Array of /Game/RPG/Blueprints/Item/S_ItemSlot Structure"))
  (bind _itemtoadd (`local.ItemToAdd`))
  (bind _itemtoadd_2 (`local.ItemToAdd`))
  (bind (_output_item _output_amount) (break `/Game/RPG/Blueprints/Item/S_ItemSlot` (`|GetArrayItem` (`local.LocalContent`) (`local.CurrentSlotID`))))
  (bind _stacksize (`/Game/RPG/Blueprints/Item/ItemsDatas/PDA_ItemDatas.StackSize` _itemtoadd))
  (set `local.ItemToAdd` Item)
  (set `local.AmountLeft` Count)
  (bind _output_get (set `local.LocalContent` InputContent))
  (for _index (range (`KismetArrayLibrary.Array_Length` _output_get))
    (set `local.CurrentSlotID` _index)
    ;[0.05098 0.05098 0.05098] Add Item to Existing Slot
    (set `local.CurrentSlotAmount` _output_amount)
    (if (and (== _output_item _itemtoadd) (< (`local.CurrentSlotAmount`) _stacksize))
      (if (<= (+ (`local.CurrentSlotAmount`) (`local.AmountLeft`)) _stacksize)
        (`KismetArrayLibrary.Array_Set` (`local.LocalContent`) (`local.CurrentSlotID`) (make `/Game/RPG/Blueprints/Item/S_ItemSlot` (`local.ItemToAdd`) (+ (`local.CurrentSlotAmount`) (`local.AmountLeft`))))
        (set `local.AmountLeft` 0)
        (break)
        (else
          (set `local.AmountLeft` (- (`local.AmountLeft`) (`/Game/RPG/Blueprints/Item/ItemsDatas/PDA_ItemDatas.StackSize` (`local.ItemToAdd`)) (`local.CurrentSlotAmount`)))
          (`KismetArrayLibrary.Array_Set` (`local.LocalContent`) (`local.CurrentSlotID`) (make `/Game/RPG/Blueprints/Item/S_ItemSlot` (`local.ItemToAdd`) (`/Game/RPG/Blueprints/Item/ItemsDatas/PDA_ItemDatas.StackSize` (`local.ItemToAdd`))))))))
  ;[0.05098 0.05098 0.05098] Add Item to New Slot
  (if (== (`local.AmountLeft`) 0)
    (`self.UpdateWidget`)
    (return "true" (`local.LocalContent`))
    (else
      (if (< (`KismetArrayLibrary.Array_Length` (`local.LocalContent`)) (`self.SlotsAmount`)) :!label _label
        (if (<= (`local.AmountLeft`) (`/Game/RPG/Blueprints/Item/ItemsDatas/PDA_ItemDatas.StackSize` (`local.ItemToAdd`)))
          (`KismetArrayLibrary.Array_Add` (`local.LocalContent`) (make `/Game/RPG/Blueprints/Item/S_ItemSlot` (`local.ItemToAdd`) (`local.AmountLeft`)))
          (`self.UpdateWidget`)
          (return "true" (`local.LocalContent`))
          (else
            (`KismetArrayLibrary.Array_Add` (`local.LocalContent`) (make `/Game/RPG/Blueprints/Item/S_ItemSlot` _itemtoadd_2 (`/Game/RPG/Blueprints/Item/ItemsDatas/PDA_ItemDatas.StackSize` _itemtoadd_2)))
            (set `local.AmountLeft` (- (`local.AmountLeft`) (`/Game/RPG/Blueprints/Item/ItemsDatas/PDA_ItemDatas.StackSize` (`local.ItemToAdd`))))
            (if (== (`local.AmountLeft`) 0)
              (`self.UpdateWidget`)
              (return "true" (`local.LocalContent`))
              (else
                (goto _label)))))
        (else
          (`self.UpdateWidget`)
          (return "false" (`local.LocalContent`)))))))

(fn `CanAdd`
  (params (Items :type "Array of /Game/RPG/Blueprints/Item/S_ItemSlot Structure"))
  (returns (CanAddAll :type Boolean))
  (locals (CanAdd :type Boolean) (LocalContent :type "Array of /Game/RPG/Blueprints/Item/S_ItemSlot Structure"))
  (set `local.CanAdd` true)
  (set `local.LocalContent` (`self.Content`))
  (for _array_element Items
    (bind (_bool _outputcontent) (`self.AddItemToSpecificContent` (break `/Game/RPG/Blueprints/Item/S_ItemSlot` _array_element) (`.Amount_7_E08AD9B3421E831788A24AA7FF7CCAA7` (break `/Game/RPG/Blueprints/Item/S_ItemSlot` _array_element)) (`local.LocalContent`)))
    (set `local.LocalContent` _outputcontent)
    (if (not _bool)
      (set `local.CanAdd` false)
      (break)))
  (return (`local.CanAdd`)))

(fn `CanRemove`
  (params (Item :type "/Game/RPG/Blueprints/Item/ItemsDatas/PDA_ItemDatas Object Reference") (Amount :type Integer))
  (returns (CanRemove :type Boolean) (InventoryCount :type Integer))
  (locals (ItemToCheck :type "/Game/RPG/Blueprints/Item/ItemsDatas/PDA_ItemDatas Object Reference") (AmountToCheck :type Integer))
  (set `local.ItemToCheck` Item)
  (set `local.AmountToCheck` Amount)
  (bind _inventorycount (`self.GetItemAmount` (`local.ItemToCheck`)))
  (return (<= (`local.AmountToCheck`) _inventorycount) _inventorycount))

(fn `Equip`
  (params (ItemDatas :type "/Game/RPG/Blueprints/Item/ItemsDatas/PDA_ItemDatas Object Reference") (Slot :type "/Game/RPG/UI/Menu/Inventory/WBP_EquipmentSlot Object Reference"))
  (returns (EquippedSuccessfully :type Boolean))
  (locals (EquipmentSlot :type "/Game/RPG/UI/Menu/Inventory/WBP_EquipmentSlot Object Reference") (EquipmentItemDatas :type "/Game/RPG/Blueprints/Item/ItemsDatas/PDA_ItemDatas Object Reference"))
  (bind _bp_player (`self.BP Player`))
  (set `local.EquipmentItemDatas` ItemDatas)
  (set `local.EquipmentSlot` Slot)
  (bind _canremove (`self.RemoveItem` (`local.EquipmentItemDatas`) 1))
  (if _canremove
    (`/Engine/EditorBlueprintResources/StandardMacros.IsValid` (`/Game/RPG/UI/Menu/Inventory/WBP_EquipmentSlot.ItemDatas` (`local.EquipmentSlot`))
      (:`Is Valid`
        (bind _unequippedsuccessfully (`self.UnEquip` (`local.EquipmentSlot`)))
        (if _unequippedsuccessfully
          _
          (else
            (`self.AddItem` (`local.EquipmentItemDatas`) 1)
            (return false))))
      (:`Is Not Valid`
        _))
    (`/Game/RPG/UI/Menu/Inventory/WBP_EquipmentSlot.Set Slot` (`local.EquipmentSlot`) (`local.EquipmentItemDatas`))
    (switch `/Game/RPG/Blueprints/Item/E_EquipmentType` (`/Game/RPG/UI/Menu/Inventory/WBP_EquipmentSlot.EquipmentType` (`local.EquipmentSlot`))
      (:`NewEnumerator0`
        (bind _aspda_armor_datas (cast `/Game/RPG/Blueprints/Item/ItemsDatas/PDA_ArmorDatas` (`local.EquipmentItemDatas`) :!label _label))
        (`/Game/RPG/Player/BP_Player.UpdateArmorPoints` _bp_player (+ (`/Game/RPG/Blueprints/Item/ItemsDatas/PDA_ArmorDatas.ArmorPoints` _aspda_armor_datas) (`/Game/RPG/Player/BP_Player.ArmorPoints` _bp_player))))
      (:`NewEnumerator1`
        (goto _label))
      (:`NewEnumerator2`
        (goto _label))
      (:`NewEnumerator3`
        (goto _label))
      (:`NewEnumerator4`
        (goto _label))
      (:`NewEnumerator5`
        _)
      (:`NewEnumerator6`
        _))
    (return true)))

(fn `GetItemAmount`
  (params (Item :type "/Game/RPG/Blueprints/Item/ItemsDatas/PDA_ItemDatas Object Reference"))
  (returns (InventoryCount :type Integer))
  (locals (ItemToCheck :type "/Game/RPG/Blueprints/Item/ItemsDatas/PDA_ItemDatas Object Reference") (AmountInInventory :type Integer))
  (set `local.ItemToCheck` Item)
  (set `local.AmountInInventory` 0)
  (for _array_element (`self.Content`)
    (if (== (break `/Game/RPG/Blueprints/Item/S_ItemSlot` _array_element) (`local.ItemToCheck`))
      (set `local.AmountInInventory` (+ (`local.AmountInInventory`) (`.Amount_7_E08AD9B3421E831788A24AA7FF7CCAA7` (break `/Game/RPG/Blueprints/Item/S_ItemSlot` _array_element))))))
  (return (`local.AmountInInventory`)))

(fn `RemoveItem`
  (params (Item :type "/Game/RPG/Blueprints/Item/ItemsDatas/PDA_ItemDatas Object Reference") (Amount :type Integer))
  (returns (CanRemove :type Boolean) (InventoryAmount :type Integer))
  (locals (ItemToRemove :type "/Game/RPG/Blueprints/Item/ItemsDatas/PDA_ItemDatas Object Reference") (AmoutLeft :type Integer) (CurrentSlotAmount :type Integer) (CurrentSlotIndex :type Integer) (SlotsToRemove :type "Array of Integer") (ReversedContent :type "Array of /Game/RPG/Blueprints/Item/S_ItemSlot Structure"))
  (bind _reversedcontent (`local.ReversedContent`))
  (bind _output_get (set `local.ItemToRemove` Item))
  (set `local.AmoutLeft` Amount)
  ;[0.05098 0.05098 0.05098] Check if the Item can be Removed
  (bind (_canremove _inventorycount) (`self.CanRemove` _output_get Amount))
  (if _canremove
    (`KismetArrayLibrary.Array_Clear` (`local.SlotsToRemove`))
    (bind _output_get_2 (set `local.ReversedContent` (`self.Content`)))
    (`KismetArrayLibrary.Array_Reverse` _output_get_2)
    (for (_array_element _array_index) (`local.ReversedContent`)
      (set `local.CurrentSlotAmount` (`.Amount_7_E08AD9B3421E831788A24AA7FF7CCAA7` (break `/Game/RPG/Blueprints/Item/S_ItemSlot` _array_element)))
      (set `local.CurrentSlotIndex` _array_index)
      (if (== (break `/Game/RPG/Blueprints/Item/S_ItemSlot` _array_element) (`local.ItemToRemove`))
        (if (>= (`local.AmoutLeft`) (`local.CurrentSlotAmount`))
          ;[0.05098 0.05098 0.05098] Remove Slot
          (set `local.AmoutLeft` (- (`local.AmoutLeft`) (`local.CurrentSlotAmount`)))
          (`KismetArrayLibrary.Array_Add` (`local.SlotsToRemove`) (`local.CurrentSlotIndex`))
          (else
            ;[0.05098 0.05098 0.05098] Remove some Items of a Slot
            (`KismetArrayLibrary.Array_Set` (`local.ReversedContent`) (`local.CurrentSlotIndex`) (make `/Game/RPG/Blueprints/Item/S_ItemSlot` (`local.ItemToRemove`) (- (`local.CurrentSlotAmount`) (`local.AmoutLeft`))))
            (break)))))
    ;[0.05098 0.05098 0.05098] Remove Slots to Remove
    (for (_array_element_2 _array_index_2) (`local.SlotsToRemove`)
      (`KismetArrayLibrary.Array_Remove` (`local.ReversedContent`) (- _array_element_2 _array_index_2)))
    (`KismetArrayLibrary.Array_Reverse` _reversedcontent)
    (set `self.Content` _reversedcontent)
    (`self.UpdateWidget`)
    (bind _inventorycount_2 (`self.GetItemAmount` (`local.ItemToRemove`)))
    (return true _inventorycount_2)
    (else
      (return false _inventorycount))))

(fn `UnEquip`
  (params (Slot :type "/Game/RPG/UI/Menu/Inventory/WBP_EquipmentSlot Object Reference"))
  (returns (UnequippedSuccessfully :type Boolean))
  (locals (EquipmentSlot :type "/Game/RPG/UI/Menu/Inventory/WBP_EquipmentSlot Object Reference"))
  (bind _bp_player (`self.BP Player`))
  (bind _output_get (set `local.EquipmentSlot` Slot))
  (bind _bool (`self.AddItem` (`/Game/RPG/UI/Menu/Inventory/WBP_EquipmentSlot.ItemDatas` _output_get) 1))
  (if _bool
    (switch `/Game/RPG/Blueprints/Item/E_EquipmentType` (`/Game/RPG/UI/Menu/Inventory/WBP_EquipmentSlot.EquipmentType` (`local.EquipmentSlot`))
      (:`NewEnumerator0`
        (bind _aspda_armor_datas (cast `/Game/RPG/Blueprints/Item/ItemsDatas/PDA_ArmorDatas` (`/Game/RPG/UI/Menu/Inventory/WBP_EquipmentSlot.ItemDatas` (`local.EquipmentSlot`)) :!label _label))
        (`/Game/RPG/Player/BP_Player.UpdateArmorPoints` _bp_player (- (`/Game/RPG/Player/BP_Player.ArmorPoints` _bp_player) (`/Game/RPG/Blueprints/Item/ItemsDatas/PDA_ArmorDatas.ArmorPoints` _aspda_armor_datas))))
      (:`NewEnumerator1`
        (goto _label))
      (:`NewEnumerator2`
        (goto _label))
      (:`NewEnumerator3`
        (goto _label))
      (:`NewEnumerator4`
        (goto _label))
      (:`NewEnumerator5`
        _)
      (:`NewEnumerator6`
        _))
    (`/Game/RPG/UI/Menu/Inventory/WBP_EquipmentSlot.ResetSlot` (`local.EquipmentSlot`))
    ;[1 0 0] TODO
    (`KismetSystemLibrary.PrintString` "Show mesh on player"))
  (return _bool))

(fn `UpdateWidget`
  (`/Game/RPG/UI/Menu/Inventory/WBP_Inventory.UpdateInventory` (`self.WBP_Inventory`) (`self.Content`))
  (`/Game/RPG/Blueprints/QuestsSystem/BP_QuestsManager.CheckCollectObjectives` (`/Game/RPG/Player/BP_Player.QuestsManager` (`self.BP Player`))))