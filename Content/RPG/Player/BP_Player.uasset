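; BP_Player is the RPG player character, holding health, armor, stamina, money, experience and level, and able to toggle into a bat form.
; Stat functions update their values and push them to the in-game HUD widget through the player controller.
; AddExp loops through level-ups, with each level's requirement growing exponentially.
; TransformIntoBat uses capsule height to pick the form, swapping meshes, jump, gravity and sprint, while a timeline lerps camera boom length.
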(event `self.ReceiveBeginPlay`
  (bind _aspc_player (cast `/Game/RPG/_Common/PC_Player` (`GameplayStatics.GetPlayerController` 0)))
  (set `self.PC Player` _aspc_player)
  (`self.UpdateHealth` (`self.MaxHealth`))
  (`self.UpdateArmorPoints` (`self.ArmorPoints`))
  (`self.UpdateStamina` (`self.MaxStamina`))
  (bind _returnvalue (`GameplayStatics.GetActorOfClass` "/Game/RPG/Blueprints/QuestsSystem/QuestsManager.QuestsManager_C"))
  (set `self.QuestsManager` _returnvalue)
  (`/Game/RPG/UI/InGame/WBP_InGame.UpdateMoney` (`/Game/RPG/_Common/PC_Player.WBP_InGame` (`self.PC Player`)) (`self.Money`))
  (`self.CalculateCurrentLevelExp`)
  (`/Game/RPG/UI/InGame/WBP_InGame.UpdateExp` (`/Game/RPG/_Common/PC_Player.WBP_InGame` (`self.PC Player`)) (`self.Exp`) (`self.CurrentLevelExp`))
  (`/Game/RPG/UI/InGame/WBP_InGame.UpdateLevel` (`/Game/RPG/_Common/PC_Player.WBP_InGame` (`self.PC Player`)) (`self.Level`))
  (`TimelineComponent.SetPlayRate` (`self.CameraLerp`) 3.0)
  (`SceneComponent.SetHiddenInGame` (`self.Bat`) true false)
  (`SceneComponent.SetHiddenInGame` (`self.Mesh`) false false))

(event `ChangeCameraPos`
  (params (`Reverse?` :type Boolean))
  (if `Reverse?`
    (bind (_direction _alpha) (`Timeline|CameraLerp` :!via `ReverseFromEnd` :!label _label)
      (:`Update`
        (set `SpringArmComponent.TargetArmLength` (`KismetMathLibrary.Lerp` 400.0 200.0 _alpha) (`self.CameraBoom`))))
    (else
      (goto _label :!via `PlayFromStart`))))

(fn `AddExp`
  (params (Exp :type "Float (double-precision)"))
  (bind _output_get (set `self.Exp` (+ Exp (`self.Exp`))))
  (`/Game/RPG/UI/InGame/WBP_InGame.UpdateExp` (`/Game/RPG/_Common/PC_Player.WBP_InGame` (`self.PC Player`)) _output_get (`self.CurrentLevelExp`))
  (if (>= _output_get (`self.CurrentLevelExp`)) :!label _label
    (set `self.Exp` (- (`self.Exp`) (`self.CurrentLevelExp`)))
    (bind _result (`/Engine/EditorBlueprintResources/StandardMacros.IncrementInt` (`self.Level`))
      (:`  `
        (`/Game/RPG/UI/InGame/WBP_InGame.UpdateLevel` (`/Game/RPG/_Common/PC_Player.WBP_InGame` (`self.PC Player`)) _result)
        (`self.CalculateCurrentLevelExp`)
        (`/Game/RPG/UI/InGame/WBP_InGame.UpdateExp` (`/Game/RPG/_Common/PC_Player.WBP_InGame` (`self.PC Player`)) (`self.Exp`) (`self.CurrentLevelExp`))
        (goto _label)))))

(fn `AddMoney`
  (params (Money :type "Float (double-precision)"))
  (bind _output_get (set `self.Money` (+ Money (`self.Money`))))
  (`/Game/RPG/UI/InGame/WBP_InGame.UpdateMoney` (`/Game/RPG/_Common/PC_Player.WBP_InGame` (`self.PC Player`)) _output_get))

(fn `CalculateCurrentLevelExp`
  (set `self.CurrentLevelExp` (* (`self.BaseLevelExp`) (`KismetMathLibrary.MultiplyMultiply_FloatFloat` (`self.LevelExpMultiplier`) (`KismetMathLibrary.Conv_IntToDouble` (`self.Level`))))))

(fn `RemoveMoney`
  (params (Money :type "Float (double-precision)"))
  (bind _output_get (set `self.Money` (- Money (`self.Money`))))
  (`/Game/RPG/UI/InGame/WBP_InGame.UpdateMoney` (`/Game/RPG/_Common/PC_Player.WBP_InGame` (`self.PC Player`)) _output_get))

(fn `TransformIntoBat`
  (bind _charactermovement (`self.CharacterMovement`))
  (bind _charactermovement_2 (`self.CharacterMovement`))
  (if (> (`CapsuleComponent.CapsuleHalfHeight` (`self.CapsuleComponent`)) 50.0)
    (`CapsuleComponent.SetCapsuleHalfHeight` (`self.CapsuleComponent`) 10.0 true)
    (`self.ChangeCameraPos` false)
    (`SceneComponent.SetHiddenInGame` (`self.Bat`) false false)
    (`SceneComponent.SetHiddenInGame` (`self.Mesh`) true false)
    (set `CharacterMovementComponent.JumpZVelocity` (/ (`CharacterMovementComponent.JumpZVelocity` _charactermovement_2) 1.5) _charactermovement_2)
    (set `CharacterMovementComponent.GravityScale` 1.3 _charactermovement_2)
    (set `self.CanSprint` false)
    (else
      (`CapsuleComponent.SetCapsuleHalfHeight` (`self.CapsuleComponent`) 90.0 true)
      (`self.ChangeCameraPos` true)
      (`SceneComponent.SetHiddenInGame` (`self.Bat`) true false)
      (`SceneComponent.SetHiddenInGame` (`self.Mesh`) false false)
      (set `CharacterMovementComponent.JumpZVelocity` (* (`CharacterMovementComponent.JumpZVelocity` _charactermovement) 1.5) _charactermovement)
      (set `CharacterMovementComponent.GravityScale` 1.75 _charactermovement)
      (set `self.CanSprint` true))))

(fn `UpdateArmorPoints`
  (params (ArmorPoints :type "Float (double-precision)"))
  (bind _output_get (set `self.ArmorPoints` ArmorPoints))
  (`/Game/RPG/UI/InGame/WBP_InGame.UpdateArmorPoints` (`/Game/RPG/_Common/PC_Player.WBP_InGame` (`self.PC Player`)) _output_get))

(fn `UpdateHealth`
  (params (Health :type "Float (double-precision)"))
  (if (<= Health (`self.MaxHealth`))
    (bind _output_get (set `self.CurrentHealth` Health))
    (else
      (set `self.CurrentHealth` (`self.MaxHealth`))))
  (`/Game/RPG/UI/InGame/WBP_InGame.UpdateHealth` (`/Game/RPG/_Common/PC_Player.WBP_InGame` (`self.PC Player`)) _output_get (`self.MaxHealth`)))

(fn `UpdateStamina`
  (params (CurrentStamina :type "Float (double-precision)"))
  (set `self.CurrentStamina` CurrentStamina)
  (`/Game/RPG/UI/InGame/WBP_InGame.UpdateStamina` (`/Game/RPG/_Common/PC_Player.WBP_InGame` (`self.PC Player`)) (`self.CurrentStamina`) (`self.MaxStamina`)))

(fn `UserConstructionScript`)